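; Player controller for RainbowProject that moves the player's BP_PlayerShape pawn through Enhanced Input.
; BeginPlay adds the IMC_RainbowDefault mapping context and caches the cast pawn.
; IA_Move offsets the pawn in world XY by the input scaled by its CurrentSpeed, without sweep or delta-time scaling.
; Raw WASD key events set a NewLocation vector that nothing reads.
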(event `self.ReceiveBeginPlay`
  (bind _returnvalue (subsystem `EnhancedInputLocalPlayerSubsystem`))
  ;[0.05098 0.05098 0.05098] Add Mapping Context
  (`/Engine/EditorBlueprintResources/StandardMacros.IsValid` _returnvalue
    (:`Is Valid`
      (`EnhancedInputSubsystemInterface.AddMappingContext` _returnvalue "/Game/RainbowProject/Input/IMC_RainbowDefault.IMC_RainbowDefault" 0 (struct))
      (bind _asbp_player_shape (cast `/Game/RainbowProject/BP_PlayerShape` (`GameplayStatics.GetPlayerPawn` 0)))
      (set `self.As BP Player Shape` _asbp_player_shape))))

(event `EnhancedInput|/Game/RainbowProject/Input/IA_Move`
  (params (ActionValue :type "Vector2D Structure") (ElapsedSeconds :type "Float (double-precision)") (TriggeredSeconds :type "Float (double-precision)") (InputAction :type "InputAction Object Reference" :default "/Game/RainbowProject/Input/IA_Move.IA_Move"))
  (:`Triggered`
    (`self.K2_AddActorWorldOffset` (`GameplayStatics.GetPlayerPawn` 0) (* (`PlayerShape.CurrentSpeed` (`self.As BP Player Shape`)) (`KismetMathLibrary.MakeVector` ActionValue_X ActionValue_Y)) false false)))

(event `Key|A`
  (params (Key :type "Key Structure"))
  (:`Pressed`
    (set `self.NewLocation` (0.0 10.0 0.0))))

(event `Key|D`
  (params (Key :type "Key Structure"))
  (:`Pressed`
    (set `self.NewLocation` (0.0 -10.0 0.0))))

(event `Key|W`
  (params (Key :type "Key Structure"))
  (:`Pressed`
    (set `self.NewLocation` (-10.0 0.0 0.0))))

(event `Key|S`
  (params (Key :type "Key Structure"))
  (:`Pressed`
    (set `self.NewLocation` (10.0 0.0 0.0))))

(fn `UserConstructionScript`)